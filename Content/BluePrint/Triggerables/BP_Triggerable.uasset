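; Base-style triggerable actor that reacts when characters enter or leave its Box_Trigger volume.
; Begin and end overlap events pass the other actor through ShouldReact, which accepts only Character classes and their children.
; Accepted actors are forwarded to the Overlap and Unoverlaped custom events, which currently just print the actor's display name.
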(event `Overlap`
  (params (OtherActor :type "Actor Object Reference"))
  (`KismetSystemLibrary.PrintString` (`KismetStringLibrary.Concat_StrStr` "Overlapped Actor: " (`KismetSystemLibrary.GetDisplayName` OtherActor))))

(event `self.Box_Trigger.OnComponentBeginOverlap`
  (params (OverlappedComponent :type "PrimitiveComponent Object Reference") (OtherActor :type "Actor Object Reference") (OtherComp :type "PrimitiveComponent Object Reference") (OtherBodyIndex :type Integer) (bFromSweep :type Boolean) (SweepResult :type "HitResult Structure (by ref)"))
  (bind _shouldreact (`self.Should_React` OtherActor))
  (if _shouldreact
    (`self.Overlap` OtherActor)))

(event `self.Box_Trigger.OnComponentEndOverlap`
  (params (OverlappedComponent :type "PrimitiveComponent Object Reference") (OtherActor :type "Actor Object Reference") (OtherComp :type "PrimitiveComponent Object Reference") (OtherBodyIndex :type Integer))
  (bind _shouldreact (`self.Should_React` OtherActor))
  (if _shouldreact
    (`self.Unoverlaped` OtherActor)))

(event `Unoverlaped`
  (params (OtherActor :type "Actor Object Reference"))
  (`KismetSystemLibrary.PrintString` (`KismetStringLibrary.Concat_StrStr` "Unoverlapped Actor: " (`KismetSystemLibrary.GetDisplayName` OtherActor))))

(fn `Should_React`
  (params (In_Actor :type "Actor Object Reference"))
  (returns (ShouldReact :type Boolean))
  (return (`KismetMathLibrary.ClassIsChildOf` (`GameplayStatics.GetObjectClass` In_Actor) "/Script/Engine.Character")))

(fn `UserConstructionScript`)